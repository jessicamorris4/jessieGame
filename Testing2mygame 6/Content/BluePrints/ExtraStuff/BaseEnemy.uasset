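; Base enemy character that chases the player by calling AI MoveTo every Tick unless stunned.
; A capsule hit on the player character triggers its PlayerKnockBack along the enemy's forward vector, then briefly halts the enemy on cooldown.
; Its knockback event stuns it and decrements Health, destroying it once Health is at or below the player's Str, otherwise launching it along the player's forward vector.
; Stun and cooldown share one flag, cleared after a delay.
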(event OnComponentHit(CapsuleComponent)
  (params (HitComponent :type Primitive%20Component%20Object%20Reference) (OtherActor :type Actor%20Object%20Reference) (OtherComp :type Primitive%20Component%20Object%20Reference) (NormalImpulse :type Vector :default "0, 0, 0") (Hit :type Hit%20Result%20Structure%20%28by%20ref%29))
  ;[0.3473 0.9552 1] WHAT HAPPENS WHEN THE CHARACTER AND THE ENEMEY OVERLAP
  (bind _ascharacter (Utilities|Casting|CastTocharacter OtherActor))
  (Default|PlayerKnockBack _ascharacter (Transformation|GetActorForwardVector))
  (CallFunction|CoolDown))

(event Custom|knockback
  ;[0.3473 0.9552 1] KNOCK BACK AND THE DYSTROYING OF ENEMIES
  (CallFunction|Stunned)
  (bind _ascharacter (Utilities|Casting|CastTocharacter (Game|Player|GetPlayerPawn 0)))
  (Variables|Default|SetHealth (- (Variables|Default|GetHealth) 1))
  (if (<= (Variables|Default|GetHealth) (Variables|/Game/BluePrints/character.character_C|GetStr _ascharacter))
    (Actor|DestroyActor)
    (else
      (Character|LaunchCharacter (* (Variables|/Game/BluePrints/character.character_C|GetForwardVector _ascharacter) "1000.000000,1000.000000,1000.000000") false false))))

(event Custom|Stunned
  ;[0.0488 1 0] STUNNING THE ENEMY
  (Variables|Default|Setenemystunned true)
  (Components|Movement|StopMovementImmediately (Variables|Character|GetCharacterMovement))
  (Utilities|FlowControl|Delay 2.0)
  (Variables|Default|Setenemystunned false))

(event Custom|CoolDown
  ;[0.3473 0.9552 1] COOL DOWN FUNCTION
  (Variables|Default|Setenemystunned true)
  (Components|Movement|StopMovementImmediately (Variables|Character|GetCharacterMovement))
  (Utilities|FlowControl|Delay 1.0)
  (Variables|Default|Setenemystunned false))

(event EventBeginPlay)

(event Collision|EventActorBeginOverlap
  (params (OtherActor :type Actor%20Object%20Reference)))

(event EventTick
  (params (DeltaSeconds :type Float%20%28single-precision%29))
  ;[1 0.4553 0] Moving the character to something
  (if (Variables|Default|Getenemystunned)
    (Development|PrintString "enemy stunned false")
    (else
      (AI|AIMoveTo self "0, 0, 0" (Game|Player|GetPlayerPawn 0) 5.0 false))))

(fn ConstructionScript)